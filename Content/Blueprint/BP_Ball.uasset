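; BP_Ball is a bouncing ball that moves itself along a direction vector initialized from its starting rotation.
; Each tick it sweeps forward, and on a blocking hit it reflects off the surface with Z flattened, turns to face the new direction and speeds up slightly.
; Hitting BP_Player blends the player's last direction into the ball's heading.
; Overlapping a KillZVolume calls the Dead dispatcher and destroys the ball.
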(event `self.ReceiveBeginPlay`
  (set `self.Direction` (`KismetMathLibrary.Conv_RotatorToVector` (`self.K2_GetActorRotation`))))

(event `self.ReceiveActorBeginOverlap`
  (params (OtherActor :type "Actor Object Reference"))
  (cast `KillZVolume` OtherActor)
  (`self.Dead`)
  (`self.K2_DestroyActor`))

(event `self.ReceiveTick`
  (params (DeltaSeconds :type "Float (single-precision)"))
  (bind _sweephitresult (`self.K2_AddActorWorldOffset` (* (* (`self.Direction`) (`self.Speed`)) DeltaSeconds) true))
  (bind (_bblockinghit _binitialoverlap _time _distance _location _impactpoint _normal) (`GameplayStatics.BreakHitResult` _sweephitresult))
  (if _bblockinghit
    (bind (_returnvalue_x _returnvalue_y) (`KismetMathLibrary.BreakVector` (`KismetMathLibrary.GetReflectionVector` (`self.Direction`) _normal)))
    (bind _output_get (set `self.Direction` (`KismetMathLibrary.MakeVector` _returnvalue_x _returnvalue_y)))
    (`self.K2_SetActorRotation` (`KismetMathLibrary.Conv_VectorToRotator` _output_get))
    (set `self.Speed` (+ (`self.Speed`) 0.2))))

(event `self.Sphere.OnComponentHit`
  (params (HitComponent :type "PrimitiveComponent Object Reference") (OtherActor :type "Actor Object Reference") (OtherComp :type "PrimitiveComponent Object Reference") (NormalImpulse :type "Vector Structure") (Hit :type "HitResult Structure (by ref)"))
  (bind _asbp_player (cast `/Game/Blueprint/BP_Player` OtherActor))
  (set `self.Direction` (`KismetMathLibrary.Normal` (+ (`KismetMathLibrary.Normal` (`/Game/Blueprint/BP_Player.LastDirection` _asbp_player)) (`self.Direction`)))))

(fn `UserConstructionScript`)