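; BP_Player is the player actor in a ball game with lives, moving sideways along the Y axis with sweep from the Move Right axis.
; It spawns a BP_Ball at SpawnPointBall on BeginPlay and binds to its Dead event.
; Each death costs one HP, then either respawns a ball or shows a lose widget at zero.
; P or Escape shows the GamePause_WD widget, created once and cached.
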(event `self.ReceiveBeginPlay`
  (`self.Spawn Ball`))

(event `InputAxis|Move Right`
  (params (AxisValue :type "Float (single-precision)"))
  (bind _output_get (set `self.LastDirection` (`KismetMathLibrary.MakeVector` 0.0 (* AxisValue (`self.speed`) (`GameplayStatics.GetWorldDeltaSeconds`)))))
  (`self.K2_AddActorWorldOffset` _output_get true))

(event `Spawn Ball`
  (bind _spawn_pointball (`self.Spawn PointBall`))
  (bind _returnvalue (`|SpawnActorFromClass` "/Game/Blueprint/BP_Ball.BP_Ball_C" (`KismetMathLibrary.MakeTransform` (`SceneComponent.K2_GetComponentLocation` _spawn_pointball) (`SceneComponent.K2_GetComponentRotation` _spawn_pointball)) "Undefined" "OverrideRootScale" null null))
  (add `/Game/Blueprint/BP_Ball.Dead` _returnvalue (delegate `OnDead Event`)))

(event `OnDead Event`
  (set `self.HP` (- (`self.HP`) 1))
  (if (<= (`self.HP`) 0)
    (`/Engine/EditorBlueprintResources/StandardMacros.IsValid` (`self.lose`)
      (:`Is Valid`
        _)
      (:`Is Not Valid`
        (bind _returnvalue (`|CreateWidget` "/Game/UI/LoseMenu/LoseMenu_WD.LoseMenu_WD_C"))))
    (`UserWidget.AddToViewport` _returnvalue 0)
    (else
      (`self.Spawn Ball`))))

(event `Key|P`
  (params (Key :type "Key Structure"))
  (:`Pressed`
    (`/Engine/EditorBlueprintResources/StandardMacros.IsValid` (`self.pause`) :!label _label
      (:`Is Valid`
        _)
      (:`Is Not Valid`
        (bind _returnvalue (`|CreateWidget` "/Game/UI/PauseMenu/GamePause_WD.GamePause_WD_C"))
        (bind _output_get (set `self.pause` _returnvalue))))
    (`UserWidget.AddToViewport` _output_get 0)))

(event `Key|Escape`
  (params (Key :type "Key Structure"))
  (:`Pressed`
    (goto _label)))

(fn `UserConstructionScript`)