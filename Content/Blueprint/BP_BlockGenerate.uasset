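; BP_BlockGenerate is a generator actor that lays out a flat grid of BP_Block actors when play begins.
; Nested loops over X and Y place each block at the generator's location plus the loop indices times Size, leaving height unchanged.
; Blocks always spawn regardless of collision, and the construction script is empty, so all generation happens at runtime.
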(event `self.ReceiveBeginPlay`
  (for _index (range (+ (`self.x`) 1))
    (for _index_2 (range (+ (`self.y`) 1))
      (`|SpawnActorFromClass` "/Game/Blueprint/BP_Block.BP_Block_C" (`KismetMathLibrary.MakeTransform` (+ (`self.K2_GetActorLocation`) (`KismetMathLibrary.MakeVector` (* _index (`self.size`)) (* _index_2 (`self.size`))))) "AlwaysSpawn" "OverrideRootScale" null null))))

(fn `UserConstructionScript`)